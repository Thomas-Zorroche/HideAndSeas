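; Procedural level builder that streams in a start room and one right-to-left room when play begins.
; CreateLevel makes a named streaming level instance at NextSpawn, loads and shows it, and stores it as CurrentLevel.
; Once the start room is shown, its exit transform becomes the next spawn point, chaining the second room.
; Rooms are sorted first and requested by type, though the random lookup in GetRandomRoomByType is left unconnected.
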(event `self.ReceiveBeginPlay`
  (`self.SortAllLevel`)
  (bind _current_level (`self.CreateLevel` (`self.GetRandomRoomByType` (enumliteral `RoomType` "START")) "Start"))
  (add `LevelStreaming.OnLevelShown` _current_level (delegate `OnStartingLevelShown`)))

(event `OnStartingLevelShown`
  (bind _returnvalue (`self.GetExitTransform` (`self.CurrentLevel`)))
  (set `self.NextSpawn` _returnvalue)
  (`self.CreateLevel` (`self.GetRandomRoomByType` (enumliteral `RoomType` "RIGHTTOLEFT")) "level2"))

(fn `CreateLevel`
  (params (Target :type "LevelStreaming Object Reference") (UniqueInstanceName :type String))
  (returns (`Current Level` :type "LevelStreaming Object Reference"))
  (locals (LevelToSpawn :type "LevelStreaming Object Reference") (UniqueName :type String :default "level2"))
  (bind _returnvalue (`LevelStreaming.CreateInstance` Target UniqueInstanceName))
  (set `LevelStreaming.LevelTransform` (`self.NextSpawn`) _returnvalue)
  (set `LevelStreaming.bShouldBeLoaded` true _returnvalue)
  (set `LevelStreaming.bShouldBeVisible` true _returnvalue)
  (bind _output_get (set `self.CurrentLevel` _returnvalue))
  (return _output_get))

(fn `UserConstructionScript`)