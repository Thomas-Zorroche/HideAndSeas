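; Player controller for boat navigation that switches between the sailed boat and a fog-of-war world map.
; On BeginPlay it spawns the map pawn and fog actor, caches the boat and islands container, and adds a compass widget.
; A looping timer reveals fog around the boat and updates its map marker.
; Toggle input toggles island, boat and fog visibility, resets map controls, then flip-flops possession, cursor and compass updates.
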(event `self.ReceiveBeginPlay`
  ;[1 1 1] Initialize Boat and CameraWorldMap variables
  (bind _returnvalue (`|SpawnActorFromClass` "/Game/UI/WorldMap/BP_WorldMapPawn.BP_WorldMapPawn_C" (`KismetMathLibrary.MakeTransform` (0.0 0.0 0.0)) "AlwaysSpawn" "OverrideRootScale" null null))
  (set `self.CameraWorldMap` _returnvalue)
  (bind _returnvalue_2 (`|SpawnActorFromClass` "/Game/UI/WorldMap/BP_FogWorldMap.BP_FogWorldMap_C" (`KismetMathLibrary.MakeTransform` (0.0 0.0 0.0)) "AlwaysSpawn" "OverrideRootScale" null 1.207106 null)) ; 1 + (srqt(2) - 1) / 2 = 1,207106
  (set `self.FogWorldMap` _returnvalue_2)
  (bind _asflying_boat_test (cast `/Game/Blueprints/Navigation/FlyingBoatTest` (`self.K2_GetPawn`)))
  (set `self.Boat` _asflying_boat_test)
  (`KismetSystemLibrary.K2_SetTimerDelegate` (delegate `UpdateFogEvent`) (`self.UpdateFogFrequency`) true)
  (bind _returnvalue_3 (`|CreateWidget` "/Game/UI/Navigation/Widget_Compass.Widget_Compass_C" self))
  (bind _output_get (set `self.CompassUI` _returnvalue_3))
  (`UserWidget.AddToViewport` _output_get 0)
  (bind _asgame_instance (cast `/Game/GameInstance` (`GameplayStatics.GetGameInstance`)))
  (set `self.IslandsContainer` (`/Game/GameInstance.IslandsContainer` _asgame_instance)))

(event `UpdateFogEvent`
  (bind _fogworldmap (`self.FogWorldMap`))
  (bind _returnvalue (`self.K2_GetActorLocation` (`self.Boat`)))
  ;[1 1 1] UpdateFogEvent
  (`/Game/UI/WorldMap/BP_FogWorldMap.RevealArea` _fogworldmap "NewEnumerator1" _returnvalue 0)
  (`/Game/UI/WorldMap/BP_FogWorldMap.UpdateBoatMarker` _fogworldmap _returnvalue))

(event `InputAction|ToggleWorldMap`
  (params (Key :type "Key Structure"))
  ;[1 1 1] Switch between boat and world map
  (:`Pressed`
    (`self.SwitchPawn`)))

(fn `UserConstructionScript`)