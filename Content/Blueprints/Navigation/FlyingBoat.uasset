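; Player-controlled flying sailboat that spawns at the current island's boat position and opens the island level on interact when near one.
; Each tick applies inertial yaw and physics thrust, weakened when sails are furled, with a speed cap based on wind alignment.
; Wing extension scales lift in air or rising wind, with temporary extra forward force when airborne.
; A flag shows wind direction; input also drives the camera.
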(event `self.ReceiveBeginPlay`
  (`self.SpawnBoatInPlace`))

(event `InputAction|Interact`
  (params (Key :type "Key Structure"))
  ;[0.6349 0.2499 1] Landing
  (:`Pressed`
    (if (`self.NearIsland`)
      (bind _ashide_and_seas_game_instance (cast `/Game/HideAndSeas_GameInstance` (`GameplayStatics.GetGameInstance`)))
      (`/Game/HideAndSeas_GameInstance.OpenIslandLevel` _ashide_and_seas_game_instance))))

(event `InputAxis|LookUp`
  (params (AxisValue :type "Float (single-precision)"))
  ;[1 1 1] Camera Controller
  (`self.AddControllerYawInput` AxisValue))

(event `self.ReceiveTick`
  (params (DeltaSeconds :type "Float (single-precision)"))
  ;[1 1 1] Every Frame
  (`self.RotateFlag`)
  (`self.AddRotation` DeltaSeconds)
  (`self.AddForceXY` DeltaSeconds
    (:`NewParam`
      (`self.AddForceZ` DeltaSeconds
        (:`output`
          ;[1 1 1] TEMP
          (`self.AddForwardForceInAir` DeltaSeconds))))))

(event `InputAxis|TurnCamera`
  (params (AxisValue :type "Float (single-precision)"))
  ;[1 1 1] Camera Controller
  (`self.AddControllerPitchInput` AxisValue))

(event `InputAxis|TurnBoat`
  (params (AxisValue :type "Float (single-precision)"))
  (bind _turnspeed (`self.TurnSpeed`))
  (bind _maxturnspeed (`self.MaxTurnSpeed`))
  (bind _maxturnspeed_2 (`self.MaxTurnSpeed`))
  ;[0.1914 0.7044 1] Turn Boat
  (if (and (== AxisValue 0.0) (> (`KismetMathLibrary.Abs` (`self.AccumulatedRotation`)) 0.04))
    (set `self.AccumulatedRotation` (`KismetMathLibrary.FClamp` (- (`self.AccumulatedRotation`) (* (`self.Inertia`) (`KismetMathLibrary.SignOfFloat` (`self.AccumulatedRotation`)))) (* _maxturnspeed_2 -1.0) _maxturnspeed_2))
    (else
      (set `self.AccumulatedRotation` (`KismetMathLibrary.FClamp` (+ (`KismetMathLibrary.MapRangeClamped` AxisValue -1.0 1.0 (* _turnspeed -1.0) _turnspeed) (`self.AccumulatedRotation`)) (* _maxturnspeed -1.0) _maxturnspeed)))))

(event `InputAxis|InteractWing`
  (params (AxisValue :type "Float (single-precision)"))
  (bind _rwing (`self.RWing`))
  (bind _lwing (`self.LWing`))
  (bind (_relativelocation_x _relativelocation_y) (`KismetMathLibrary.BreakVector` (`SceneComponent.RelativeLocation` _lwing)))
  (bind (_relativelocation_x_2 _relativelocation_y_2) (`KismetMathLibrary.BreakVector` (`SceneComponent.RelativeLocation` (`self.RWing`))))
  (bind (_relativelocation_x_3 _relativelocation_y_3) (`KismetMathLibrary.BreakVector` (`SceneComponent.RelativeLocation` _rwing)))
  ;[1 0.7732 0.06453] Wings
  (if (!= AxisValue 0.0)
    (`SceneComponent.K2_SetRelativeLocation` _lwing (`KismetMathLibrary.MakeVector` 0.0 (`KismetMathLibrary.FClamp` (+ AxisValue _relativelocation_y) -201.0 0.0)) false false)
    (`SceneComponent.K2_SetRelativeLocation` _rwing (`KismetMathLibrary.MakeVector` 0.0 (`KismetMathLibrary.FClamp` (+ (* AxisValue -1.0) _relativelocation_y_3) 0.0 201.0)) false false)
    (set `self.WingsAmount` (`KismetMathLibrary.MapRangeClamped` _relativelocation_y_2 0.0 200.0 0.0 1.0))))

(event `InputAction|InteractSails`
  (params (Key :type "Key Structure"))
  (bind _sails (`self.Sails`))
  (bind _sails_2 (`self.Sails`))
  (bind (_returnvalue_x _returnvalue_y) (`KismetMathLibrary.BreakVector` (`SceneComponent.K2_GetComponentScale` _sails)))
  (bind (_returnvalue_x_2 _returnvalue_y_2) (`KismetMathLibrary.BreakVector` (`SceneComponent.K2_GetComponentScale` _sails_2)))
  ;[1 0.3162 0.2465] Sails
  (:`Pressed`
    (`/Engine/EditorBlueprintResources/StandardMacros.FlipFlop`
      (:`A`
        (`SceneComponent.SetWorldScale3D` _sails_2 (`KismetMathLibrary.MakeVector` _returnvalue_x_2 _returnvalue_y_2 0.1))
        (set `self.AreSailsDeployed` false))
      (:`B`
        (`SceneComponent.SetWorldScale3D` _sails (`KismetMathLibrary.MakeVector` _returnvalue_x _returnvalue_y 3.0))
        (set `self.AreSailsDeployed` true)))))

(fn `getWindAlignement`
  (returns (alignement :type "Float (double-precision)"))
  (return (`KismetMathLibrary.Dot_VectorVector` (`KismetMathLibrary.Normal` (`self.GetActorForwardVector`)) (`KismetMathLibrary.Normal` (`self.WindDirection`)))))

(fn `GetXYSpeed`
  (returns (ReturnValue :type "Float (double-precision)"))
  (bind (_returnvalue_x _returnvalue_y) (`KismetMathLibrary.BreakVector` (`self.GetVelocity`)))
  (return (`KismetMathLibrary.VSize` (`KismetMathLibrary.MakeVector` _returnvalue_x _returnvalue_y))))

(fn `UserConstructionScript`)