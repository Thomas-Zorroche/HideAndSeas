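; BP_Island is an island actor that shows an interaction prompt when the flying boat comes within range.
; A Sphere overlap with FlyingBoat3 creates Interact_UI, guarded by an Opened flag, and leaving removes the first top-level instance found by class search.
; The construction script randomizes the root's integer scale independently on each axis, and a Backspace key event prints a debug message.
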(event `self.Sphere.OnComponentBeginOverlap`
  (params (OverlappedComponent :type "PrimitiveComponent Object Reference") (OtherActor :type "Actor Object Reference") (OtherComp :type "PrimitiveComponent Object Reference") (OtherBodyIndex :type Integer) (bFromSweep :type Boolean) (SweepResult :type "HitResult Structure (by ref)"))
  (cast `/Game/Blueprints/Navigation/FlyingBoat3` OtherActor)
  (if (not (`self.Opened`))
    (bind _returnvalue (`|CreateWidget` "/Game/UI/Interact_UI.Interact_UI_C"))
    (`UserWidget.AddToViewport` _returnvalue 0)
    (set `self.Opened` true)))

(event `self.Sphere.OnComponentEndOverlap`
  (params (OverlappedComponent :type "PrimitiveComponent Object Reference") (OtherActor :type "Actor Object Reference") (OtherComp :type "PrimitiveComponent Object Reference") (OtherBodyIndex :type Integer))
  (cast `/Game/Blueprints/Navigation/FlyingBoat3` OtherActor)
  (bind _foundwidgets (`WidgetBlueprintLibrary.GetAllWidgetsOfClass` "/Game/UI/Interact_UI.Interact_UI_C"))
  (if (`KismetArrayLibrary.Array_IsValidIndex` _foundwidgets)
    (`Widget.RemoveFromParent` (`|GetArrayItem` _foundwidgets))
    (set `self.Opened` false)))

(event `Key|BackSpace`
  (params (Key :type "Key Structure"))
  (:`Pressed`
    (`KismetSystemLibrary.PrintString` "Hello")))

(fn `UserConstructionScript`
  (bind _returnvalue (`KismetMathLibrary.Conv_IntToDouble` (`KismetMathLibrary.RandomIntegerInRange` 5 10)))
  (`SceneComponent.SetWorldScale3D` (`self.DefaultSceneRoot`) (`KismetMathLibrary.MakeVector` _returnvalue _returnvalue _returnvalue)))