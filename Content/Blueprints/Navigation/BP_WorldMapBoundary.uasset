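; World map boundary that wraps a FlyingBoat3 to the opposite side of the map when it leaves the volume.
; End overlap on the collision box casts the exiting actor to FlyingBoat3 and passes it to TeleportBoat.
; TeleportBoat negates whichever of X or Y has the larger magnitude, mirroring the boat across the world origin while preserving the other coordinates.
; The move is unswept, and the math assumes an origin-centered map.
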(event `self.CollisionBox.OnComponentEndOverlap`
  (params (OverlappedComponent :type "PrimitiveComponent Object Reference") (OtherActor :type "Actor Object Reference") (OtherComp :type "PrimitiveComponent Object Reference") (OtherBodyIndex :type Integer))
  (bind _asflying_boat_3 (cast `/Game/Blueprints/Navigation/FlyingBoat3` OtherActor))
  (`self.TeleportBoat` _asflying_boat_3))

(fn `UserConstructionScript`)