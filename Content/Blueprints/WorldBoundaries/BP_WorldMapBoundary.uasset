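; BP_WorldMapBoundary is a world map boundary that wraps the player's flying boat to the opposite side when it exits the collision box.
; BeginPlay caches the possessed boat's hull mesh, and only that component ending overlap triggers TeleportBoat.
; TeleportBoat negates whichever of X or Y is larger in magnitude, mirroring across the world origin while keeping Z, and moves the boat without sweeping.
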(event `self.ReceiveBeginPlay`
  (bind _asflying_boat_test (cast `/Game/Blueprints/Navigation/FlyingBoatTest` (`Controller.K2_GetPawn` (`GameplayStatics.GetPlayerController` 0))))
  (set `self.BoatMesh` (`/Game/Blueprints/Navigation/FlyingBoatTest.SM_Boat_Hull` _asflying_boat_test)))

(event `self.CollisionBox.OnComponentEndOverlap`
  (params (OverlappedComponent :type "PrimitiveComponent Object Reference") (OtherActor :type "Actor Object Reference") (OtherComp :type "PrimitiveComponent Object Reference") (OtherBodyIndex :type Integer))
  (bind _boatmesh (`self.BoatMesh`))
  (if (== OtherComp _boatmesh)
    (bind _asflying_boat_test (cast `/Game/Blueprints/Navigation/FlyingBoatTest` (`ActorComponent.GetOwner` _boatmesh)))
    (`self.TeleportBoat` _asflying_boat_test)))

(fn `UserConstructionScript`)