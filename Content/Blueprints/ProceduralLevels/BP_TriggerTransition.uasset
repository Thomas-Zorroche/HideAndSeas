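; Trigger volume for procedural level transitions that calls off attacking enemies when the top-down player character enters its box.
; On overlap, it asks the GameManager game instance's LevelManager for all enemies on the player's tile.
; Any SEnemyController in the attack state gets OnPlayerCaught, reused here to reset patrollers to patrolling.
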(event `self.Box.OnComponentBeginOverlap`
  (params (OverlappedComponent :type "PrimitiveComponent Object Reference") (OtherActor :type "Actor Object Reference") (OtherComp :type "PrimitiveComponent Object Reference") (OtherBodyIndex :type Integer) (bFromSweep :type Boolean) (SweepResult :type "HitResult Structure (by ref)"))
  (cast `/Game/Characters/TopDownCharacter/BP_TopDownCharacter` OtherActor)
  (bind _asgame_manager (cast `GameManager` (`GameplayStatics.GetGameInstance`)))
  (bind _returnvalue (`SLevelManager.GetAllEnemiesFromPlayerTile` (`GameManager.LevelManager` _asgame_manager)))
  ;[1 1 1] Just reset patroller to patrol state
  (for _array_element _returnvalue
    (bind _assenemy_controller (cast `SEnemyController` (`AIBlueprintHelperLibrary.GetAIController` _array_element)))
    (if (`|EnumEquality` (`SEnemyController.State` _assenemy_controller) "ATTACK")
      (`SEnemyController.OnPlayerCaught` _assenemy_controller))))

(fn `UserConstructionScript`)