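; BP_CampFire is a campfire light for procedural levels that pulses its point light while switched on.
; The light on and off events set an On flag that gates the Tick update.
; Each tick drives intensity from an absolute sine of game time since creation, clamped to the upper range for a subtle pulse.
; The off event only stops these updates and does not itself change the intensity.
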(event `self.OnLightTurnOff`
  (set `self.On` false))

(event `self.OnLightTurnOn`
  (set `self.On` true))

(event `self.ReceiveTick`
  (params (DeltaSeconds :type "Float (single-precision)"))
  (if (`self.On`)
    (`LightComponent.SetIntensity` (`self.PointLight`) (* (`KismetMathLibrary.FClamp` (`KismetMathLibrary.Abs` (`KismetMathLibrary.Sin` (`self.GetGameTimeSinceCreation`))) 0.7) 50000.0))))

(fn `UserConstructionScript`)