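; BP_Jail is a procedural-level jail actor that sends the player to its location when they are caught.
; On player start it binds a jail event to the player-caught event.
; That event fetches all enemies from the player's tile via the GameManager's LevelManager, teleports the player to the jail's root, then calls OnPlayerCaught on each enemy's AI controller.
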(event `self.OnPlayerStart`
  (add `self.PlayerCaught` (delegate `JailEvent`)))

(event `JailEvent`
  (bind _asgame_manager (cast `GameManager` (`GameplayStatics.GetGameInstance`)))
  (bind _returnvalue (`SLevelManager.GetAllEnemiesFromPlayerTile` (`GameManager.LevelManager` _asgame_manager)))
  (`self.SetPlayerToJail`)
  (for _array_element _returnvalue
    (bind _assenemy_controller (cast `SEnemyController` (`AIBlueprintHelperLibrary.GetAIController` _array_element)))
    (`SEnemyController.OnPlayerCaught` _assenemy_controller)))

(fn `SetPlayerToJail`
  (`self.K2_SetActorLocation` (`GameplayStatics.GetPlayerCharacter` 0) (`SceneComponent.K2_GetComponentLocation` (`self.DefaultSceneRoot`)) false true))

(fn `UserConstructionScript`)