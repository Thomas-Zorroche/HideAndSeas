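; Player start actor for procedural levels that places the player and doubles as the jail they return to when caught.
; On its start event it teleports player character 0 to its root component's location, then binds JailEvent to the player-caught event.
; When JailEvent fires, SetPlayerToJail repeats the same teleport back to that location.
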(event `self.OnPlayerStart`
  (`self.K2_SetActorLocation` (`GameplayStatics.GetPlayerCharacter` 0) (`SceneComponent.K2_GetComponentLocation` (`self.DefaultSceneRoot`)) false true)
  (add `self.PlayerCaught` (delegate `JailEvent`)))

(event `JailEvent`
  (`self.SetPlayerToJail`))

(fn `SetPlayerToJail`
  (`self.K2_SetActorLocation` (`GameplayStatics.GetPlayerCharacter` 0) (`SceneComponent.K2_GetComponentLocation` (`self.DefaultSceneRoot`)) false true))

(fn `UserConstructionScript`)