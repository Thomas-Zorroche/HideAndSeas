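; Pressure-tile trigger that completes a procedural-level room when the top-down player stands on it for CompletionTime.
; Entering starts a timer, sinks the tile and ramps up lights and Niagara particles on timelines.
; Leaving early cancels the timer, reverses both animations and zeroes the audio AlertLevel parameter.
; On completion it locks, notifies the GameManager's LevelManager and changes the player's crystal to the current color.
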(event `AnimateTile`
  (params (Forward :type Boolean))
  (bind _tile (`self.Tile`))
  (bind (_returnvalue_x _returnvalue_y) (`KismetMathLibrary.BreakVector` (`SceneComponent.K2_GetComponentLocation` _tile)))
  (if Forward
    (bind (_direction _value) (`Timeline|Timeline_1` :!label _label)
      (:`Update`
        (`SceneComponent.K2_SetWorldLocation` _tile (`KismetMathLibrary.MakeVector` _returnvalue_x _returnvalue_y (`KismetMathLibrary.Lerp` (`self.TileInitialZ`) (- (`self.TileInitialZ`) 15.0) _value)) false false)))
    (else
      (goto _label :!via `Reverse`))))

(event `self.Box.OnComponentBeginOverlap`
  (params (OverlappedComponent :type "PrimitiveComponent Object Reference") (OtherActor :type "Actor Object Reference") (OtherComp :type "PrimitiveComponent Object Reference") (OtherBodyIndex :type Integer) (bFromSweep :type Boolean) (SweepResult :type "HitResult Structure (by ref)"))
  (cast `/Game/Characters/TopDownCharacter/BP_TopDownCharacter` OtherActor)
  (if (and (not (`self.IsPlayerInTrigger`)) (`self.PlayerCanComplete`))
    (set `self.IsPlayerInTrigger` true)
    (`GameplayStatics.PlaySound2D` "/Game/Sounds/Sfx/Sound_StoneSlide.Sound_StoneSlide" 1.0 1.0 0.0 null null)
    (bind _returnvalue (`KismetSystemLibrary.K2_SetTimerDelegate` (delegate `OnCompleteTile`) (`self.CompletionTime`)))
    (set `self.Timer` _returnvalue)
    (`self.AnimateTile` true)
    (`self.AnimateLights` true)))

(event `OnCompleteTile`
  (`KismetSystemLibrary.K2_ClearAndInvalidateTimerHandle` (`self.Timer`))
  (set `self.PlayerCanComplete` false)
  (`self.CompleteRoom`))

(event `self.Box.OnComponentEndOverlap`
  (params (OverlappedComponent :type "PrimitiveComponent Object Reference") (OtherActor :type "Actor Object Reference") (OtherComp :type "PrimitiveComponent Object Reference") (OtherBodyIndex :type Integer))
  (cast `/Game/Characters/TopDownCharacter/BP_TopDownCharacter` OtherActor)
  (if (and (`self.IsPlayerInTrigger`) (`self.PlayerCanComplete`))
    (set `self.IsPlayerInTrigger` false)
    (`KismetSystemLibrary.K2_ClearAndInvalidateTimerHandle` (`self.Timer`))
    (bind _asgame_instance (cast `/Game/GameInstance` (`GameplayStatics.GetGameInstance`)))
    (`AudioComponent.SetFloatParameter` (`/Game/GameInstance.Audio` _asgame_instance) "AlertLevel" 0.0)
    (`GameplayStatics.PlaySound2D` "/Game/Sounds/Sfx/Sound_StoneSlide.Sound_StoneSlide" 1.0 1.0 0.0 null null)
    (`self.AnimateTile` false)
    (`self.AnimateLights` false)))

(event `self.OnLightTurnOn`
  ;[1 1 1] Turn Light on and off
  (`self.LightsOn`))

(event `self.ReceiveBeginPlay`
  (`TimelineComponent.SetTimelineLength` (`self.Timeline_0`) (`self.CompletionTime`)))

(event `self.OnLightTurnOff`
  ;[1 1 1] Turn Light on and off
  (`self.LightOff`))

(event `AnimateLights`
  (params (On :type Boolean))
  (if On
    (bind (_direction _newtrack_0) (`Timeline|Timeline_0` :!label _label_2)
      (:`Update`
        (bind _returnvalue (* _newtrack_0 (`self.MaxLightIntensity`)))
        (`LightComponent.SetIntensity` (`self.PointLight1`) _returnvalue)
        (`LightComponent.SetIntensity` (`self.PointLight`) _returnvalue)
        (`self.Update Niagara Size` (* (`self.NiagaraMinSize`) _newtrack_0) (* (`self.NiagaraMaxSize`) _newtrack_0))))
    (else
      (goto _label_2 :!via `Reverse`))))

(fn `CompleteRoom`
  ;[1 1 1] Complete Level Fr
  (bind _asgame_manager (cast `GameManager` (`GameplayStatics.GetGameInstance`)))
  (`SLevelManager.CompleteRoom` (`GameManager.LevelManager` _asgame_manager) (`SceneComponent.K2_GetComponentLocation` (`self.DefaultSceneRoot`)))
  (bind _asbp_top_down_character (cast `/Game/Characters/TopDownCharacter/BP_TopDownCharacter` (`GameplayStatics.GetPlayerCharacter` 0)))
  (`/Game/Characters/TopDownCharacter/BP_TopDownCharacter.ChangeCrystal` _asbp_top_down_character (`GameManager.CurrentCrystalColor` _asgame_manager)))

(fn `Update Niagara Size`
  (params (MinSize :type "Vector2D Structure" :default (0.0 0.0)) (MaxSize :type "Vector2D Structure"))
  (bind _niagara1 (`self.Niagara1`))
  (bind _niagara (`self.Niagara`))
  (`NiagaraComponent.SetNiagaraVariableVec2` _niagara1 "MinSize" MinSize)
  (`NiagaraComponent.SetNiagaraVariableVec2` _niagara1 "MaxSize" MaxSize)
  (`NiagaraComponent.SetNiagaraVariableVec2` _niagara "MinSize" MinSize)
  (`NiagaraComponent.SetNiagaraVariableVec2` _niagara "MaxSize" MaxSize))

(fn `UserConstructionScript`
  (bind (_returnvalue_x _returnvalue_y _returnvalue_z) (`KismetMathLibrary.BreakVector` (`SceneComponent.K2_GetComponentLocation` (`self.Tile`))))
  (set `self.TileInitialZ` _returnvalue_z))