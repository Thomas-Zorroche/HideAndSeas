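; BP_Lampadaire is a lamppost actor whose light fades on or off through two custom events.
; OnLightTurnOff plays the TurnLightOn timeline forward and OnLightTurnon reverses it from the end, printing debug messages.
; The timeline's Brightness track scales both spotlights' intensity and the Emissive parameter of a dynamic material instance created on BeginPlay for the lamppost mesh.
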(event `self.OnLightTurnOff`
  (`KismetSystemLibrary.PrintString` "Light Turn Off")
  (bind (_direction _brightness) (`Timeline|TurnLightOn` :!via `PlayFromStart` :!label _label)
    (:`Update`
      (bind _returnvalue (* _brightness 50000.0))
      (`LightComponent.SetIntensity` (`self.SpotLight1`) _returnvalue)
      (`LightComponent.SetIntensity` (`self.SpotLight`) _returnvalue)
      (`MaterialInstanceDynamic.SetScalarParameterValue` (`self.Material`) "Emissive" (* _brightness 11.0)))
    (:`Finished`
      (`KismetSystemLibrary.PrintString` "Anim Finished"))))

(event `self.OnLightTurnOn`
  (`KismetSystemLibrary.PrintString` "Light Turn On")
  (goto _label :!via `ReverseFromEnd`))

(event `self.ReceiveBeginPlay`
  (bind _returnvalue (`PrimitiveComponent.CreateDynamicMaterialInstance` (`self.SM_lamppost_03`) 1 "/Game/ExternalAssets/Medieval_Village/materials/props_materials/MI_lamppost_02_Inst.MI_lamppost_02_Inst" "None"))
  (set `self.Material` _returnvalue))

(fn `UserConstructionScript`)