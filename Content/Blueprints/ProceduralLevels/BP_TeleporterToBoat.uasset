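; BP_TeleporterToBoat is an exit point in procedural levels that lets the player leave the island for the ocean level.
; A box trigger tracks whether the top-down character is inside, showing a UI_LeaveIsland prompt on entry and removing it on exit.
; When the OnPlayerAction event fires while the player is inside, it removes the prompt and calls OpenOceanLevel on the custom GameInstance.
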(event `self.Box1.OnComponentBeginOverlap`
  (params (OverlappedComponent :type "PrimitiveComponent Object Reference") (OtherActor :type "Actor Object Reference") (OtherComp :type "PrimitiveComponent Object Reference") (OtherBodyIndex :type Integer) (bFromSweep :type Boolean) (SweepResult :type "HitResult Structure (by ref)"))
  (cast `/Game/Characters/TopDownCharacter/BP_TopDownCharacter` OtherActor)
  (if (not (`self.PlayerInside`))
    (set `self.PlayerInside` true)
    (bind _returnvalue (`|CreateWidget` "/Game/UI/IslandLevel/UI_LeaveIsland.UI_LeaveIsland_C"))
    (bind _output_get (set `self.UIText` _returnvalue))
    (`UserWidget.AddToViewport` _output_get 0)))

(event `self.Box1.OnComponentEndOverlap`
  (params (OverlappedComponent :type "PrimitiveComponent Object Reference") (OtherActor :type "Actor Object Reference") (OtherComp :type "PrimitiveComponent Object Reference") (OtherBodyIndex :type Integer))
  (cast `/Game/Characters/TopDownCharacter/BP_TopDownCharacter` OtherActor)
  (set `self.PlayerInside` false)
  (`Widget.RemoveFromParent` (`self.UIText`)))

(event `/Game/Blueprints/ProceduralLevels/BI_OnAction.OnPlayerAction`
  (if (`self.PlayerInside`)
    (`Widget.RemoveFromParent` (`self.UIText`))
    (bind _asgame_instance (cast `/Game/GameInstance` (`GameplayStatics.GetGameInstance`)))
    (`/Game/GameInstance.OpenOceanLevel` _asgame_instance)))

(fn `UserConstructionScript`)