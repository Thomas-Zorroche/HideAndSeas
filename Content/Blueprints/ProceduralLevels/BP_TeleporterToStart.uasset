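; Portal actor that sends the player back to BP_Jail once the current island is finished.
; On BeginPlay it asks the GameManager's LevelManager whether the island is finished, setting its active flag and the portal material's Lit parameter to match.
; Two trigger boxes track which was entered first, so entering the second before leaving the first calls TeleportToJail, which wraps the jail move in a camera fade.
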(event `self.ReceiveBeginPlay`
  (bind _returnvalue (`PrimitiveComponent.CreateDynamicMaterialInstance` (`self.PortalPlane`) 0 "/Game/Graphics/Materials/MI_Portal.MI_Portal" "None"))
  (set `self.PortalMaterialnstance` _returnvalue)
  (bind _asgame_manager (cast `GameManager` (`GameplayStatics.GetGameInstance`)))
  (bind _levelmanager (`GameManager.LevelManager` _asgame_manager))
  (bind _returnvalue_2 (`SLevelManager.isIslandFinished` _levelmanager (`SLevelManager.CurrentIslandID` _levelmanager)))
  (bind _output_get (set `self.Activate` _returnvalue_2))
  (if _output_get
    (`self.Set Portal Intensity` 1.0)
    (else
      (`self.Set Portal Intensity` 0.0))))

(event `self.Box2.OnComponentBeginOverlap`
  (params (OverlappedComponent :type "PrimitiveComponent Object Reference") (OtherActor :type "Actor Object Reference") (OtherComp :type "PrimitiveComponent Object Reference") (OtherBodyIndex :type Integer) (bFromSweep :type Boolean) (SweepResult :type "HitResult Structure (by ref)"))
  (`/Engine/EditorBlueprintResources/StandardMacros.IsValid` (`self.FirstBoxTraversed`)
    (:`Is Valid`
      (`self.TeleportToJail` :!label _label))
    (:`Is Not Valid`
      (set `self.FirstBoxTraversed` (`self.Box2`)))))

(event `self.Box1.OnComponentBeginOverlap`
  (params (OverlappedComponent :type "PrimitiveComponent Object Reference") (OtherActor :type "Actor Object Reference") (OtherComp :type "PrimitiveComponent Object Reference") (OtherBodyIndex :type Integer) (bFromSweep :type Boolean) (SweepResult :type "HitResult Structure (by ref)"))
  (`/Engine/EditorBlueprintResources/StandardMacros.IsValid` (`self.FirstBoxTraversed`)
    (:`Is Valid`
      (goto _label))
    (:`Is Not Valid`
      (set `self.FirstBoxTraversed` (`self.Box1`)))))

(event `self.Box1.OnComponentEndOverlap`
  (params (OverlappedComponent :type "PrimitiveComponent Object Reference") (OtherActor :type "Actor Object Reference") (OtherComp :type "PrimitiveComponent Object Reference") (OtherBodyIndex :type Integer))
  (if (== (`self.Box1`) (`self.FirstBoxTraversed`))
    (set `self.FirstBoxTraversed` null :!label _label_2)))

(event `self.Box2.OnComponentEndOverlap`
  (params (OverlappedComponent :type "PrimitiveComponent Object Reference") (OtherActor :type "Actor Object Reference") (OtherComp :type "PrimitiveComponent Object Reference") (OtherBodyIndex :type Integer))
  (if (== (`self.Box2`) (`self.FirstBoxTraversed`))
    (goto _label_2)))

(fn `Set Portal Intensity`
  (params (Intensity :type "Float (double-precision)"))
  (`MaterialInstanceDynamic.SetScalarParameterValue` (`self.PortalMaterialnstance`) "Lit" Intensity))

(fn `UserConstructionScript`)