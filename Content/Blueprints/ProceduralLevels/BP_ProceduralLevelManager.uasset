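; Level manager actor that decides on BeginPlay whether the currently visited island needs a new procedural level.
; If so, it spawns a BP_SProceduralLevel generator, randomizes its LevelSize and binds to the game instance's generation-finished event.
; When that event fires, it unbinds and adds the generator's LevelData to the game instance.
; Rebuilding from existing level data is only a debug print.
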(event `self.ReceiveBeginPlay`
  (bind _ashide_and_seas_game_instance (cast `/Game/HideAndSeas_GameInstance` (`GameplayStatics.GetGameInstance`)))
  (bind _output_get (set `self.GameInstance` _ashide_and_seas_game_instance))
  (bind _mustgeneratenewprocedurallevel (`/Game/HideAndSeas_GameInstance.Get Current Visited Island Data` _output_get))
  (if _mustgeneratenewprocedurallevel
    ;[1 1 1] Generate new Level
    (bind _returnvalue (`|SpawnActorFromClass` (`self.LevelGeneratorClass`) (`KismetMathLibrary.MakeTransform` (0.0 0.0 0.0)) "Undefined" "OverrideRootScale" null null))
    (bind _asbp_sprocedural_level (cast `/Game/Blueprints/ProceduralLevels/BP_SProceduralLevel` _returnvalue))
    (bind _output_get_2 (set `self.ProceduralLevelGenerator` _asbp_sprocedural_level))
    (bind _output_get_3 (set `/Game/Blueprints/ProceduralLevels/BP_SProceduralLevel.LevelSize` (`KismetMathLibrary.RandomIntegerInRange` 6 10) _output_get_2))
    (`KismetSystemLibrary.PrintString` (`KismetStringLibrary.Concat_StrStr` "LevelSize : " (`KismetStringLibrary.Conv_IntToString` _output_get_3)) true true (struct :`R` 1.0 :`B` 0.954921 :`A` 1.0))
    ;[1 1 1] Transfer Generated Level Data to Game Instance
    (add `/Game/HideAndSeas_GameInstance.OnFinishLevelGeneration` (`self.GameInstance`) (delegate `OnFinishLevelGeneration`))
    (else
      (`KismetSystemLibrary.PrintString` "Generate Level With Level Data"))))

(event `OnFinishLevelGeneration`
  ;[1 1 1] Transfer Generated Level Data to Game Instance
  (remove `/Game/HideAndSeas_GameInstance.OnFinishLevelGeneration` (`self.GameInstance`) (delegate `OnFinishLevelGeneration`))
  (`/Game/HideAndSeas_GameInstance.AddLevelData` (`self.GameInstance`) (`/Game/Blueprints/ProceduralLevels/BP_SProceduralLevel.LevelData` (`self.ProceduralLevelGenerator`)))
  (`KismetSystemLibrary.PrintString` "LevelGenerationFinish" true true (struct :`R` 1.0 :`B` 0.856693 :`A` 1.0)))

(fn `UserConstructionScript`)