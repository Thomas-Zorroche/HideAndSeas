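; End-of-island chest that finishes the current procedural island and awards the player a crystal when opened.
; On BeginPlay it tints the crystal through a dynamic material, using the island's color from the GameInstance's LevelManager.
; Collision overlap toggles reachability and the interact widget, and the player action opens the lid and notifies the LevelManager.
; A timeline raises the crystal, then adds it to the player controller and starts a sine bob on Tick.
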(event `self.ReceiveBeginPlay`
  ;[1 1 1] Setup
  (bind _asbp_top_down_player_controller (cast `/Game/Characters/TopDownCharacter/BP_TopDownPlayerController` (`GameplayStatics.GetPlayerController` 0)))
  (bind _output_get (set `self.TopDownPlayerController` _asbp_top_down_player_controller))
  (`self.EnableInput` _output_get)
  (bind _returnvalue (`|CreateWidget` "/Game/UI/Widget_InteractChest.Widget_InteractChest_C" (`self.TopDownPlayerController`)))
  (set `self.InteractUI` _returnvalue)
  (bind _asgame_instance (cast `/Game/GameInstance` (`GameplayStatics.GetGameInstance`)))
  (set `self.GameInstance` _asgame_instance)
  (bind _returnvalue_2 (`PrimitiveComponent.CreateDynamicMaterialInstance` (`self.crystal`) 0 "/Game/Graphics/Materials/M_Crystal.M_Crystal" "None"))
  (bind _returnvalue_3 (`SLevelManager.GetCrystalColorOfCurrentIsland` (`GameManager.LevelManager` (`self.GameInstance`))))
  (bind _output_get_2 (set `self.CrystalColor` _returnvalue_3))
  (`MaterialInstanceDynamic.SetVectorParameterValue` _returnvalue_2 "Color" (`KismetMathLibrary.Conv_ColorToLinearColor` _output_get_2)))

(event `self.CollisionBox.OnComponentBeginOverlap`
  (params (OverlappedComponent :type "PrimitiveComponent Object Reference") (OtherActor :type "Actor Object Reference") (OtherComp :type "PrimitiveComponent Object Reference") (OtherBodyIndex :type Integer) (bFromSweep :type Boolean) (SweepResult :type "HitResult Structure (by ref)"))
  ;[1 1 1] Switch reachable state
  (cast `/Game/Characters/TopDownCharacter/BP_TopDownCharacter` OtherActor)
  (set `self.ChestReachable` true)
  (if (not (`self.Open`))
    (`UserWidget.AddToViewport` (`self.InteractUI`) 0)))

(event `self.CollisionBox.OnComponentEndOverlap`
  (params (OverlappedComponent :type "PrimitiveComponent Object Reference") (OtherActor :type "Actor Object Reference") (OtherComp :type "PrimitiveComponent Object Reference") (OtherBodyIndex :type Integer))
  ;[1 1 1] Switch reachable state
  (cast `/Game/Characters/TopDownCharacter/BP_TopDownCharacter` OtherActor)
  (set `self.ChestReachable` false)
  (`Widget.RemoveFromParent` (`self.InteractUI`)))

(event `/Game/Blueprints/ProceduralLevels/BI_OnAction.OnPlayerAction`
  ;[1 1 1] Open chest
  (if (and (`self.ChestReachable`) (not (`self.Open`)))
    (`Widget.RemoveFromParent` (`self.InteractUI`))
    (`SLevelManager.FinishCurrentIsland` (`GameManager.LevelManager` (`self.GameInstance`)))
    (`KismetSystemLibrary.PrintString` "Open chest")
    (`self.OpenChest`)))

(event `OpenChest`
  (bind (_returnvalue_x _returnvalue_y _returnvalue_z) (`KismetMathLibrary.BreakVector` (`SceneComponent.K2_GetComponentLocation` (`self.crystal`))))
  (bind (_returnvalue_x_2 _returnvalue_y_2 _returnvalue_z_2) (`KismetMathLibrary.BreakVector` (`SceneComponent.K2_GetComponentLocation` (`self.crystal`))))
  ;[1 1 1] Open Chest - Open Lid and translate crystal
  (set `self.CrystalBaseZ` _returnvalue_z_2)
  (`SceneComponent.K2_AddLocalRotation` (`self.Lid`) (struct :`Roll` -90.0) false false)
  (bind (_direction _zoffset) (`Timeline|Timeline_0`)
    (:`Update`
      (`self.AnimCrystal` _zoffset))
    (:`Finished`
      (set `self.Open` true)
      (set `self.CrystalBaseZ` _returnvalue_z)
      (bind _asbp_top_down_player_controller (cast `/Game/Characters/TopDownCharacter/BP_TopDownPlayerController` (`GameplayStatics.GetPlayerController` 0)))
      (`/Game/Characters/TopDownCharacter/BP_TopDownPlayerController.AddCrystal` _asbp_top_down_player_controller (`KismetMathLibrary.Conv_ByteToInt` (`SLevelManager.CurrentIslandID` (`GameManager.LevelManager` (`self.GameInstance`)))) (`self.CrystalColor`)))))

(event `self.ReceiveTick`
  (params (DeltaSeconds :type "Float (single-precision)"))
  (bind _crystal (`self.crystal`))
  (bind (_returnvalue_x _returnvalue_y) (`KismetMathLibrary.BreakVector` (`SceneComponent.K2_GetComponentLocation` _crystal)))
  (if (`self.Open`)
    (`SceneComponent.K2_SetWorldLocation` _crystal (`KismetMathLibrary.MakeVector` _returnvalue_x _returnvalue_y (+ (`self.CrystalBaseZ`) (* (`KismetMathLibrary.Sin` (`self.GetGameTimeSinceCreation`)) 50.0))) false false)))

(fn `UserConstructionScript`)