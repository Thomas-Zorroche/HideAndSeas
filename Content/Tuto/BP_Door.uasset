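; BP_Door is a tutorial double door that opens when a Character enters its trigger box and closes when a Character leaves.
; Box overlap events filter for Characters and call InteractDoor with an open or close flag.
; InteractDoor instantly snaps both door leaves to fixed world-space yaws, with no animation, so the result ignores the actor's own rotation.
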(event `self.Box.OnComponentBeginOverlap`
  (params (OverlappedComponent :type "PrimitiveComponent Object Reference") (OtherActor :type "Actor Object Reference") (OtherComp :type "PrimitiveComponent Object Reference") (OtherBodyIndex :type Integer) (bFromSweep :type Boolean) (SweepResult :type "HitResult Structure (by ref)"))
  (cast `Character` OtherActor)
  (`self.InteractDoor` true))

(event `self.Box.OnComponentEndOverlap`
  (params (OverlappedComponent :type "PrimitiveComponent Object Reference") (OtherActor :type "Actor Object Reference") (OtherComp :type "PrimitiveComponent Object Reference") (OtherBodyIndex :type Integer))
  (cast `Character` OtherActor)
  (`self.InteractDoor` false))

(fn `InteractDoor`
  (params (Open :type Boolean))
  (bind _doorleft (`self.DoorLeft`))
  (bind _doorright (`self.DoorRight`))
  (if Open
    (`SceneComponent.K2_SetWorldRotation` _doorleft (`KismetMathLibrary.MakeRotator` 0.0 0.0 90.0) false false)
    (`SceneComponent.K2_SetWorldRotation` _doorright (`KismetMathLibrary.MakeRotator` 0.0 0.0 90.0) false false)
    (else
      (`SceneComponent.K2_SetWorldRotation` _doorleft (`KismetMathLibrary.MakeRotator` 0.0 0.0 180.0) false false)
      (`SceneComponent.K2_SetWorldRotation` _doorright (`KismetMathLibrary.MakeRotator` 0.0) false false))))

(fn `UserConstructionScript`)