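; Patrol path Blueprint that spawns an enemy and hands it a route built from the path's markers.
; When OnMarkersChanged fires with at least one marker, it spawns EnemyClass at the first marker location.
; If the spawn is a BP_Patroller with an EnemyPatrolController, it passes all marker locations to that controller and calls its OnSpawn.
; Each qualifying marker change spawns another actor, with no cleanup of earlier ones here.
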(event `self.OnMarkersChanged`
  (bind _returnvalue (`self.GetMarkersLocation`))
  (if (> (`KismetArrayLibrary.Array_Length` _returnvalue) 0)
    (bind _returnvalue_2 (`|SpawnActorFromClass` (`self.EnemyClass`) (`KismetMathLibrary.MakeTransform` (`|GetArrayItem` _returnvalue)) "Undefined" "OverrideRootScale" null null))
    (bind _asbp_patroller (cast `/Game/Characters/BP_Patroller` _returnvalue_2))
    (bind _asenemy_patrol_controller (cast `/Game/AI/EnemyPatrolController` (`AIBlueprintHelperLibrary.GetAIController` _asbp_patroller)))
    (set `/Game/AI/EnemyPatrolController.MarkersLocations` _returnvalue _asenemy_patrol_controller)
    (`/Game/AI/EnemyPatrolController.OnSpawn` _asenemy_patrol_controller)))

(fn `UserConstructionScript`)