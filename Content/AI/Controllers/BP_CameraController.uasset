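; AI controller for BP_Camera security cameras, which track a direction, watch for the player and raise the alarm.
; It runs BT_Camera with wait times from the pawn, and Tick turns the mesh and focal point along the current direction.
; Alert level drives a music parameter.
; Attacking sends ATTACK to patrollers from the camera's tile, though the loop returns after the first; catching the player resets to patrol.
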(event `self.ReceivePossess`
  (params (PossessedPawn :type "Pawn Object Reference"))
  (bind _asbp_camera (cast `/Game/Characters/Enemies/Camera/BP_Camera` PossessedPawn))
  (bind _output_get (set `self.CameraPawn` _asbp_camera))
  (`self.InitializeDirection` (`SceneComponent.GetForwardVector` (`Actor.RootComponent` _output_get))))

(event `self.LinkBehaviorTree`
  (`self.RunBehaviorTree` "/Game/AI/BT_Camera.BT_Camera")
  (bind _asbp_camera (cast `/Game/Characters/Enemies/Camera/BP_Camera` (`self.K2_GetPawn`)))
  (bind _enemycomp (`SCamera.EnemyComp` _asbp_camera))
  ;[1 1 1] Init Blackboard Wait variables
  (`BlackboardComponent.SetValueAsFloat` (`self.Blackboard`) "SearchWait" (`SEnemyComponent.SearchWait` _enemycomp))
  (`BlackboardComponent.SetValueAsFloat` (`self.Blackboard`) "PatrolWait" (`SEnemyComponent.PatrolWait` _enemycomp))
  (bind _asgame_instance (cast `/Game/GameInstance` (`GameplayStatics.GetGameInstance`)))
  (set `self.GameInstance` _asgame_instance))

(event `self.ReceiveTick`
  (params (DeltaSeconds :type "Float (single-precision)"))
  (bind _staticmesh (`/Game/Characters/Enemies/Camera/BP_Camera.StaticMesh` (`self.CameraPawn`)))
  (if (`/Game/Characters/Enemies/Camera/BP_Camera.IsEnabled` (`self.CameraPawn`))
    (`SceneComponent.K2_SetWorldRotation` _staticmesh (`KismetMathLibrary.MakeRotationFromAxes` (`self.CurrentDirection`)) false false)
    (`self.K2_SetFocalPoint` (+ (`SceneComponent.K2_GetComponentLocation` _staticmesh) (* (`SceneComponent.GetForwardVector` _staticmesh) (5000.0 5000.0 0.0))))
    (if (> (`self.AlertLevel`) 0.0)
      (`self.UpdateMusicWithAlertLevel`))))

(event `self.OnDebugStateLabelChanged`
  (params (debugStateLabel :type String))
  (bind _asbp_camera (cast `/Game/Characters/Enemies/Camera/BP_Camera` (`self.K2_GetPawn`)))
  (`TextRenderComponent.K2_SetText` (`/Game/Characters/Enemies/Camera/BP_Camera.TextRender` _asbp_camera) (`KismetTextLibrary.Conv_StringToText` debugStateLabel)))

(event `self.SetState`
  (params (State :type "AIState Enum" :default "PATROL"))
  (`self.SetAIState` State))

(event `self.OnReachMaxAngle`
  (`BlackboardComponent.SetValueAsBool` (`self.Blackboard`) "FixedPawn" true))

(event `self.OnAttack`
  (`self.WarnAllPatrollers`)
  (`/Game/Characters/Enemies/Camera/BP_Camera.OnAttack` (`self.CameraPawn`)))

(event `self.OnPlayerCaught`
  (`self.ResetOnPlayerCaught`)
  (`/Game/Characters/Enemies/Camera/BP_Camera.OnPlayerCaught` (`self.CameraPawn`))
  (`self.UpdateMusicWithAlertLevel`))

(fn `ResetOnPlayerCaught`
  (`BlackboardComponent.ClearValue` (`self.Blackboard`) "TargetActor")
  (`self.SetAlertLevel` 0.0)
  (`self.SetState` "PATROL"))

(fn `UpdateMusicWithAlertLevel`
  (`AudioComponent.SetFloatParameter` (`/Game/GameInstance.Audio` (`self.GameInstance`)) "AlertLevel" (`self.AlertLevel`)))

(fn `UserConstructionScript`
  (`parent.UserConstructionScript`))