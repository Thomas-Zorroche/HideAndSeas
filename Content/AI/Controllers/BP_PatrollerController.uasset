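; AI controller for a patroller character, which runs the BT_Patroller behavior tree when linked.
; GetNextLocation steps an index through MarkersLocations and wraps to the start, producing a looping patrol route.
; SetState forwards to SetAIState, and debug state label changes are written to the controlled BP_Patroller's TextRender.
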(event `self.LinkBehaviorTree`
  (`self.RunBehaviorTree` "/Game/AI/BT_Patroller.BT_Patroller"))

(event `self.OnDebugStateLabelChanged`
  (params (debugStateLabel :type String))
  (bind _asbp_patroller (cast `/Game/Characters/Enemies/BP_Patroller` (`self.K2_GetPawn`)))
  (`TextRenderComponent.K2_SetText` (`/Game/Characters/Enemies/BP_Patroller.TextRender` _asbp_patroller) (`KismetTextLibrary.Conv_StringToText` debugStateLabel)))

(event `/Game/AI/BI_AIState.SetState`
  (params (State :type "AIState Enum" :default "PATROL"))
  (`self.SetAIState` State))

(fn `GetNextLocation`
  (returns (Position :type "Vector Structure"))
  (bind _result (`/Engine/EditorBlueprintResources/StandardMacros.IncrementInt` (`self.CurrentMarkerIndex`))
    (:`  `
      (if (>= _result (`KismetArrayLibrary.Array_Length` (`self.MarkersLocations`)))
        (set `self.CurrentMarkerIndex` 0))
      (return (`|GetArrayItem` (`self.MarkersLocations`) (`self.CurrentMarkerIndex`))))))

(fn `UserConstructionScript`
  (`parent.UserConstructionScript`))