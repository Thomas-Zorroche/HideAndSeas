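; BP_Patroller is a patrolling character that visually reports its AI state and alert level.
; UpdateAlertLevel scales the spotlight intensity from a base value by alert amount, starting at zero alert on construction.
; UpdateState writes Patrol, Alert, Attack or Search to a debug TextRender.
; Each Tick orients that label toward the top-down player's camera using its forward vector with pitch and yaw offsets.
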(event `self.ReceiveTick`
  (params (DeltaSeconds :type "Float (single-precision)"))
  ;[1 1 1] Debug
  (`self.AlignTextWithCamera`))

(fn `UpdateAlertLevel`
  (params (Alert :type "Float (double-precision)"))
  (`LightComponent.SetIntensity` (`self.SpotLight`) (+ (* Alert 5000.0) (`self.BaseIntensityLight`))))

(fn `UpdateState`
  (params (NewParam :type "/Game/AI/E_AIState Enum" :default "NewEnumerator0"))
  (locals (Text :type Text))
  (switch `/Game/AI/E_AIState` NewParam
    (:`NewEnumerator0`
      (set `local.Text` "Patrol"))
    (:`NewEnumerator1`
      (set `local.Text` "Alert"))
    (:`NewEnumerator2`
      (set `local.Text` "Attack"))
    (:`NewEnumerator3`
      (set `local.Text` "Search")))
  (`TextRenderComponent.K2_SetText` (`self.TextRender`) (`local.Text`)))

(fn `UserConstructionScript`
  (`self.UpdateAlertLevel` 0.0))