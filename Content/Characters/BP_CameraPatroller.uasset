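; BP_CameraPatroller is a patrolling enemy character with a debug text label that shows its AI state.
; On BeginPlay it calls OnSpawn on its EnemyPatrolController.
; UpdateStateFn maps Patrol, Alert, Attack and Search states to the label text.
; Each tick, the label is rotated from the top-down player camera's forward vector, with pitch and yaw offsets, to stay readable on screen.
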(event `self.ReceiveTick`
  (params (DeltaSeconds :type "Float (single-precision)"))
  ;[1 1 1] Debug
  (`self.AlignTextWithCamera`))

(event `self.ReceiveBeginPlay`
  (bind _asenemy_patrol_controller (cast `/Game/AI/EnemyPatrolController` (`self.GetController`)))
  (`/Game/AI/EnemyPatrolController.OnSpawn` _asenemy_patrol_controller false))

(fn `UpdateStateFn`
  (params (State :type "/Game/AI/E_AIState Enum" :default "NewEnumerator0"))
  (locals (Text :type Text))
  (switch `/Game/AI/E_AIState` State
    (:`NewEnumerator0`
      (set `local.Text` "Patrol"))
    (:`NewEnumerator1`
      (set `local.Text` "Alert"))
    (:`NewEnumerator2`
      (set `local.Text` "Attack"))
    (:`NewEnumerator3`
      (set `local.Text` "Search")))
  (`TextRenderComponent.K2_SetText` (`self.TextRender`) (`local.Text`)))

(fn `UserConstructionScript`)