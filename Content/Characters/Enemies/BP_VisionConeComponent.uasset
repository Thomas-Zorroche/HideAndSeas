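; Static mesh component in the enemy characters folder that displays a vision cone on a scaled plane with the M_VisionCone material.
; Externally supplied Update calls write its world position, texture size and alert level (as completion) to the CharacterPosition material parameter collection.
; Each update also clears a render target and canvas-draws one triangle, fanning from the texture center along the given forward and right vectors.
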(event `self.ReceiveBeginPlay`
  (`self.SetStaticMesh` "/Game/StarterContent/Shapes/Shape_Plane.Shape_Plane")
  (`self.SetMaterial` 0 "/Game/Graphics/Materials/M_VisionCone.M_VisionCone")
  (`self.SetRelativeScale3D` (12.0 12.0 12.0)))

(fn `Update`
  (params (ForwardVector :type "Vector Structure") (RightVector :type "Vector Structure") (AlertLevel :type "Float (double-precision)"))
  (`|ExecutionSequence`
    (:`then_0`
      (`KismetMaterialLibrary.SetVectorParameterValue` "/Game/Graphics/Materials/characterPosition.characterPosition" "characterPosition" (`KismetMathLibrary.Conv_VectorToLinearColor` (`self.K2_GetComponentLocation`)))
      (`KismetMaterialLibrary.SetScalarParameterValue` "/Game/Graphics/Materials/characterPosition.characterPosition" "textureSize" (`self.textureSize`))
      (`KismetMaterialLibrary.SetScalarParameterValue` "/Game/Graphics/Materials/characterPosition.characterPosition" "completion" AlertLevel))
    (:`then_1`
      (`self.PrepateTriangles` ForwardVector RightVector))
    (:`then_2`
      (`self.UpdateRenderTarget`))))