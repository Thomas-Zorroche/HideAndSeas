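; BP_Camera is an AI-driven camera enemy with a text label that turns to match the player's view.
; On BeginPlay it tells its BP_CameraController to link the behavior tree, leaving decision logic outside this Blueprint.
; Every Tick, AlignTextWithCamera billboards the TextRender using the BP_TopDownCharacter camera's forward vector, with a pitch offset and a half-turn in yaw.
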(event `self.ReceiveBeginPlay`
  (bind _asbp_camera_controller (cast `/Game/AI/Controllers/BP_CameraController` (`self.GetController`)))
  (`SEnemyController.LinkBehaviorTree` _asbp_camera_controller))

(event `self.ReceiveTick`
  (params (DeltaSeconds :type "Float (single-precision)"))
  (`self.AlignTextWithCamera`))

(fn `UserConstructionScript`)