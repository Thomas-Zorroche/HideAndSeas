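; Enemy character Blueprint that handles the visual side of an enemy: a debug state label and a spotlight.
; Label change events set the TextRender text, and light level change events set the SpotLight intensity.
; Every Tick, AlignTextWithCamera turns the label toward the top-down player's camera, using its forward vector with flipped yaw and a pitch offset.
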(event `self.ReceiveTick`
  (params (DeltaSeconds :type "Float (single-precision)"))
  (`self.AlignTextWithCamera`))

(event `self.OnDebugStateLabelChanged`
  (params (debugStateLabel :type String))
  (`TextRenderComponent.K2_SetText` (`self.TextRender`) (`KismetTextLibrary.Conv_StringToText` debugStateLabel)))

(event `self.OnLightLevelChanged`
  (params (currentLightIntensity :type "Float (single-precision)"))
  (`LightComponent.SetIntensity` (`self.SpotLight`) currentLightIntensity))

(fn `UserConstructionScript`)