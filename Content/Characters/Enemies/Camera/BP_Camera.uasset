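; Security camera enemy that watches for the player through AI sight and a visible vision cone.
; BeginPlay links the controller's behavior tree and sizes the cone from EnemyComp; the cone clears when outside the player's tile.
; Attack and caught events recolor the dynamic material and spotlight, while disabling or room completion turns off sight and hides the cone.
; Construction enforces a minimum height; Tick turns state-colored text toward the player camera.
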(event `self.ReceiveBeginPlay`
  (bind _asbp_camera_controller (cast `/Game/AI/Controllers/BP_CameraController` (`self.GetController`)))
  (`SEnemyController.LinkBehaviorTree` _asbp_camera_controller)
  (`self.SetVisionConeData`)
  (bind _returnvalue (`PrimitiveComponent.CreateDynamicMaterialInstance` (`self.StaticMesh`) 0 "/Game/Graphics/Materials/PBR_Emissive/MI_Camera.MI_Camera" "None"))
  (set `self.Material` _returnvalue)
  (if (not (`self.IsEnabled`))
    (`self.StopLogic`)))

(event `self.ReceiveTick`
  (params (DeltaSeconds :type "Float (single-precision)"))
  (`self.AlignTextWithCamera`))

(event `self.OnPlayerTileChanged`
  (bind _output_get (set `/Game/Characters/Enemies/BP_VisionConeComponent.OwnerInsidePlayerTile` (`self.InsidePlayerTile`) (`self.ConeVision`)))
  (if (not _output_get)
    (`/Game/Characters/Enemies/BP_VisionConeComponent.Clear` (`self.ConeVision`))))

(event `OnAttack`
  (`MaterialInstanceDynamic.SetVectorParameterValue` (`self.Material`) "EmissiveColor" (struct :`R` 1.0 :`B` 0.538267 :`A` 1.0))
  (`LightComponent.SetLightColor` (`self.SpotLight`) (struct :`R` 0.895833 :`G` 0.01728 :`A` 1.0) true))

(event `OnPlayerCaught`
  (`MaterialInstanceDynamic.SetVectorParameterValue` (`self.Material`) "EmissiveColor" (struct :`R` 1.0 :`G` 1.0 :`B` 1.0 :`A` 1.0))
  (`LightComponent.SetLightColor` (`self.SpotLight`) (struct :`R` 1.0 :`G` 0.47451 :`B` 0.090196 :`A` 1.0) true))

(event `self.OnRoomComplete`
  (set `self.IsEnabled` false)
  (`self.StopLogic`))

(fn `UserConstructionScript`
  (bind _defaultsceneroot (`self.DefaultSceneRoot`))
  (bind (_returnvalue_x _returnvalue_y _returnvalue_z) (`KismetMathLibrary.BreakVector` (`SceneComponent.K2_GetComponentLocation` _defaultsceneroot)))
  (bind (_returnvalue_x_2 _returnvalue_y_2 _returnvalue_z_2) (`KismetMathLibrary.BreakVector` (`SceneComponent.K2_GetComponentLocation` (`self.DefaultSceneRoot`))))
  (if (< _returnvalue_z_2 100.0)
    (`SceneComponent.K2_SetWorldLocation` _defaultsceneroot (`KismetMathLibrary.MakeVector` _returnvalue_x _returnvalue_y (+ _returnvalue_z (`KismetMathLibrary.Abs` (- _returnvalue_z 100.0)) 5.0)) false false)))