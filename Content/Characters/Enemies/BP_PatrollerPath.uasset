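; BP_PatrollerPath spawns a patrolling enemy and hands it the path defined by its markers.
; When markers change and at least one exists, it spawns the patroller class at the first marker, setting its default transform and enemy component and updating its vision cone.
; It then notifies the patroller's AI controller of the component, passes all marker locations and links the behavior tree.
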(event `self.OnMarkersChanged`
  (bind _returnvalue (`self.GetMarkersLocation`))
  (bind _output (`|GetArrayItem` _returnvalue))
  (if (> (`KismetArrayLibrary.Array_Length` _returnvalue) 0)
    (bind _returnvalue_2 (`|SpawnActorFromClass` (`self.PatrollerClass`) (`KismetMathLibrary.MakeTransform` _output) "Undefined" "OverrideRootScale" null null))
    (bind _asbp_patroller (cast `/Game/Characters/Enemies/BP_Patroller` _returnvalue_2))
    (set `/Game/Characters/Enemies/BP_Patroller.DefaultTransform` (`KismetMathLibrary.MakeTransform` _output) _asbp_patroller)
    (set `SPatroller.EnemyComp` (`self.EnemyComp`) _asbp_patroller)
    (`/Game/Characters/Enemies/BP_Patroller.UpdateVisionCone` _asbp_patroller)
    (bind _asbp_patroller_controller (cast `/Game/AI/Controllers/BP_PatrollerController` (`AIBlueprintHelperLibrary.GetAIController` _asbp_patroller)))
    (`SEnemyController.OnEnemyComponentChanged` _asbp_patroller_controller)
    (set `/Game/AI/Controllers/BP_PatrollerController.MarkersLocations` _returnvalue _asbp_patroller_controller)
    (`SEnemyController.LinkBehaviorTree` _asbp_patroller_controller)))

(fn `UserConstructionScript`)